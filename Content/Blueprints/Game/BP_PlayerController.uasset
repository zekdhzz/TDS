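; Player controller that creates the in-game UI and links its inventory stats widget to the controlled BP_Character.
; BeginPlay adds the widget to the viewport, then binds inventory events and fills weapon and ammo slots through InitWeaponWidget, which binds again.
; Possession reinitializes the character's inventory component from its current slots, without calling the widget directly.
; Unpossession unbinds the widget's events, falling back to the controlled pawn if the given one is invalid.
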(event Custom|InitWeaponWidget
  (params (Weapons :type Array%20of%20Weapon%20Slot%20Structures) (Ammo :type Array%20of%20Ammo%20Slot%20Structures))
  (bind _ingamewidget (Variables|Default|GetIngameWidget))
  (bind _bpw_inventorystatswidget (Variables|/Game/UI/Widget/BPW_UI.BPW_UI_C|GetBPW_InventoryStatsWidget _ingamewidget))
  (Utilities|IsValid _ingamewidget
    (:Is%20Valid
      (bind _asbp_character (Utilities|Casting|CastToBP_Character (Pawn|GetControlledPawn)))
      (Default|BindInventoryEvents _bpw_inventorystatswidget _asbp_character)
      (Default|InitInventorySlots _bpw_inventorystatswidget Weapons Ammo)
      (Development|PrintString "Init Weapon Widget"))))

(event EventBeginPlay
  (Development|PrintString "creating ui")
  (bind _returnvalue (UserInterface|CreateWidget "/Game/UI/Widget/BPW_UI.BPW_UI_C" self))
  (Variables|Default|SetIngameWidget _returnvalue)
  (UserInterface|Viewport|AddtoViewport _returnvalue 0)
  (bind _asbp_character (Utilities|Casting|CastToBP_Character (Pawn|GetControlledPawn)))
  (Default|BindInventoryEvents (Variables|/Game/UI/Widget/BPW_UI.BPW_UI_C|GetBPW_InventoryStatsWidget (Variables|Default|GetIngameWidget)) _asbp_character)
  (CallFunction|InitWeaponWidget (Variables|/Script/TDS.TDSInventoryComponent|GetWeaponSlots (Variables|/Script/TDS.TDSCharacter|GetInventoryComponent _asbp_character)) (Variables|/Script/TDS.TDSInventoryComponent|GetAmmoSlots (Variables|/Script/TDS.TDSCharacter|GetInventoryComponent _asbp_character))))

(event EventPossess
  (params (PossessedPawn :type Pawn%20Object%20Reference))
  (bind _asbp_character (Utilities|Casting|CastToBP_Character PossessedPawn))
  (Class|TDSInventoryComponent|InitInventory (Variables|/Script/TDS.TDSCharacter|GetInventoryComponent _asbp_character) (Variables|/Script/TDS.TDSInventoryComponent|GetWeaponSlots (Variables|/Script/TDS.TDSCharacter|GetInventoryComponent _asbp_character)) (Variables|/Script/TDS.TDSInventoryComponent|GetAmmoSlots (Variables|/Script/TDS.TDSCharacter|GetInventoryComponent _asbp_character))))

(event EventUnPossess
  (params (UnpossessedPawn :type Pawn%20Object%20Reference))
  (CallFunction|UnbindWidget UnpossessedPawn))

(fn ConstructionScript)

(fn UnbindWidget
  (params (traget :type Object%20Object%20Reference))
  (bind _ingamewidget (Variables|Default|GetIngameWidget))
  (Utilities|IsValid traget
    (:Is%20Valid
      (LocalVariables|SettargetToUnbind traget))
    (:Is%20Not%20Valid
      (LocalVariables|SettargetToUnbind (Pawn|GetControlledPawn))))
  (Utilities|IsValid _ingamewidget
    (:Is%20Valid
      (bind _asbp_character (Utilities|Casting|CastToBP_Character (LocalVariables|GettargetToUnbind)))
      (Default|UnbindAllEvents (Variables|/Game/UI/Widget/BPW_UI.BPW_UI_C|GetBPW_InventoryStatsWidget _ingamewidget) _asbp_character))))