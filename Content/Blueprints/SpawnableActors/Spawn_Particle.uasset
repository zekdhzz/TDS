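; Spawnable actor that plays a particle effect and a sound at its location, either once or on repeat.
; On BeginPlay it activates the VFX component, plays the sound and waits for the Interval delay.
; With IsLoop set it deactivates the effect and restarts the cycle; otherwise it destroys itself.
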(event EventBeginPlay
  (Components|Activation|Activate (Variables|Default|GetVFX) false :!label _label)
  (Audio|PlaySoundatLocation (Variables|Default|GetSound) (Transformation|GetActorLocation) "0, 0, 0" 1.0 1.0 0.0 0 0 0)
  (Utilities|FlowControl|Delay (Variables|Default|Getinterval))
  (if (Variables|Default|GetisLoop)
    (Components|Activation|Deactivate (Variables|Default|GetVFX))
    (goto _label)
    (else
      (Actor|DestroyActor))))

(event Collision|EventActorBeginOverlap
  (params (OtherActor :type Actor%20Object%20Reference)))

(event EventTick
  (params (DeltaSeconds :type Float%20%28single-precision%29)))

(fn ConstructionScript)