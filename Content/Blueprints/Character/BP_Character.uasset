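; Top-down shooter character Blueprint that links weapon events to its animation Blueprint and adds weapon test keys.
; Number keys select a named starting weapon or toggle the weapon debug state.
; BeginPlay caches the TDS_AnimBP instance, which the fire and reload events then drive.
; Helper functions play a world camera shake at the top-down camera and draw debug arrows for facing, velocity and cursor aim.
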(event EventWeaponFireStartBP
  (params (Anim :type Anim%20Montage%20Object%20Reference))
  (Default|Fire (Variables|Default|GetCharAnimInstance) Anim))

(event EventBeginPlay
  (bind _astds_anim_bp (Utilities|Casting|CastToTDS_AnimBP (Components|SkeletalMesh|GetAnimInstance (Variables|Character|GetMesh))))
  (Variables|Default|SetCharAnimInstance _astds_anim_bp))

(event EventWeaponReloadStartBP
  (params (Anim :type Anim%20Montage%20Object%20Reference))
  (Default|Reload (Variables|Default|GetCharAnimInstance) Anim))

(event EventWeaponReloadEndBP
  (params (bIsSuccess :type Boolean))
  (Default|Reload (Variables|Default|GetCharAnimInstance)))

(event Input|KeyboardEvents|0
  (params (Key :type Key%20Structure :default "None"))
  (bind _returnvalue (Class|TDSCharacter|GetWeaponDebugState))
  (:Pressed
    (Class|TDSCharacter|SetWeaponDebugState (not _returnvalue))
    (Development|PrintString (Utilities|String|ToString(Boolean) _returnvalue))))

(event Input|KeyboardEvents|1
  (params (Key :type Key%20Structure :default "None"))
  (:Pressed
    (Class|TDSCharacter|SetInitWeaponName "Rifle_v1.0")))

(event Input|KeyboardEvents|2
  (params (Key :type Key%20Structure :default "None"))
  (:Pressed
    (Class|TDSCharacter|SetInitWeaponName "ShotGun_v1.0")))

(event Input|KeyboardEvents|3
  (params (Key :type Key%20Structure :default "None"))
  (:Pressed
    (Class|TDSCharacter|SetInitWeaponName "GrenadeLauncher_v1.0")))

(event Input|KeyboardEvents|4
  (params (Key :type Key%20Structure :default "None"))
  (:Pressed
    (Class|TDSCharacter|SetInitWeaponName "SniperRifle_v1.0")))

(fn ConstructionScript)

(fn CameraShakeEvent
  (Camera|PlayWorldCameraShake "/Game/Blueprints/Game/BP_ShakeCamera.BP_ShakeCamera_C" (Transformation|GetWorldLocation (Variables|Default|GetTopDownCameraComponent)) 0.0 3e+01))

(fn DebugRotationVector
  (bind _returnvalue (Transformation|GetActorLocation))
  (bind _returnvalue_2 (Transformation|GetActorLocation))
  (bind _returnvalue_3 (Game|GetPlayerController 0))
  (bind _returnvalue_4 (Transformation|GetActorLocation))
  (bind (_worldlocation _worlddirection) (Game|Player|ConvertMouseLocationToWorldSpace _returnvalue_3))
  (bind _returnvalue_5 (* _worlddirection 5e+02))
  (bind _returnvalue_6 (+ _worldlocation _returnvalue_5))
  (Rendering|Debug|DrawDebugArrow _returnvalue_2 (+ _returnvalue_2 (* (Transformation|GetActorForwardVector) 5e+02)) 2.0 "(R=0.000000,G=0.906250,B=0.221442,A=1.000000)" 0.0 4.0)
  (Rendering|Debug|DrawDebugArrow _returnvalue (+ _returnvalue (* (Math|Vector|Normalize (Transformation|GetVelocity)) 5e+02)) 2.0 "(R=0.906250,G=0.000000,B=0.778725,A=1.000000)" 0.0 4.0)
  (Rendering|Debug|DrawDebugArrow (Transformation|GetActorLocation) (.location (.HitResult (Game|Player|GetHitResultUnderCursorbyChannel (Game|GetPlayerController 0) "TraceTypeQuery3" false))) 2.0 "(R=0.000000,G=0.000000,B=0.000000,A=1.000000)" 0.0 4.0)
  (Rendering|Debug|DrawDebugArrow (Math|Vector|MakeVector (.x _returnvalue_4) (.y _returnvalue_4) (.z _returnvalue_4)) (Math|Vector|MakeVector (.x _returnvalue_6) (.y _returnvalue_6) (.z _returnvalue_4)) 2.0 "(R=1.000000,G=0.000000,B=0.024068,A=1.000000)" 0.0 4.0))